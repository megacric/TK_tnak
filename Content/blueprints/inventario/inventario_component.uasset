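; Inventory component that holds items in an array sized to a slot count on BeginPlay and toggles an inventory window.
; The toggle creates the widget on the player controller's HUD canvas with UI-only, locked-mouse input, or removes it and restores game-only input.
; Additem handles only items not flagged usable, writing them over the slot found by matching a placeholder struct with quantity 2, without stacking.
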(event `self.ReceiveBeginPlay`
  (`self.prepararinventario`))

(fn `additem`
  (params (item :type "/Game/blueprints/inventario/E_inventario Structure"))
  (returns (funciona :type Boolean))
  (if (not (`.usable_8_9ED78214449DAE6773D025A3DE5F5C09` (break `/Game/blueprints/inventario/E_intems` (break `/Game/blueprints/inventario/E_inventario` item))))
    (`self.usable` (`local.item`))
    (return true)))

(fn `inventariofun`
  (`self.ventana inventario`
    (:`then`
      (`Widget.RemoveFromParent` (`self.ventana inventario`))
      (set `self.ventana inventario` null)
      (`WidgetBlueprintLibrary.SetInputMode_GameOnly` (`GameplayStatics.GetPlayerController` 0)))
    (:`else`
      (bind _returnvalue (`|CreateWidget` "/Game/blueprints/inventario/interfaz_inventario/VENTANA.VENTANA_C" null self))
      (set `self.ventana inventario` _returnvalue)
      (bind _asplayer_controller_bp (cast `/Game/blueprints/inventario/interfaz_inventario/player_controllerBp` (`GameplayStatics.GetPlayerController` 0)))
      (bind _returnvalue_2 (`CanvasPanel.AddChildToCanvas` (`/Game/blueprints/inventario/interfaz_inventario/HUD.HUDcanvas` (`/Game/blueprints/inventario/interfaz_inventario/player_controllerBp.Hud wid` _asplayer_controller_bp)) (`self.ventana inventario`)))
      (`CanvasPanelSlot.SetAutoSize` _returnvalue_2 true)
      (`CanvasPanelSlot.SetAlignment` _returnvalue_2 (0.5 0.5))
      (`CanvasPanelSlot.SetAnchors` _returnvalue_2 (`self.anclas`))
      (`WidgetBlueprintLibrary.SetInputMode_UIOnlyEx` (`GameplayStatics.GetPlayerController` 0) null "LockAlways"))))

(fn `prepararinventario`
  (`KismetArrayLibrary.Array_Resize` (`self.itemsinvetario`) (`self.espacios`)))

(fn `usable`
  (params (itemtoadd :type "/Game/blueprints/inventario/E_inventario Structure"))
  (bind _itemsinvetario (`self.itemsinvetario`))
  (`KismetArrayLibrary.Array_Set` _itemsinvetario (`KismetArrayLibrary.Array_Find` _itemsinvetario (make `/Game/blueprints/inventario/E_inventario` (struct) 2)) itemtoadd))