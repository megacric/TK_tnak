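; Player character for a 2D flipbook side-scroller, with movement, wall jumps, dash, melee attack, teleport and inventory.
; Tick picks a movement state that the axis input turns into flipbook and scale changes.
; Wall jumps sphere-trace and launch off the hit normal; dashing briefly shrinks the capsule.
; Attacks sweep a cube along a spline via timeline; overlaps lower player health or enemy health variables stored on this Blueprint.
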(event `self.ReceiveBeginPlay`
  (`SceneComponent.SetVisibility` (`self.Cube`) false false))

(event `InputAxis|Adelante`
  (params (AxisValue :type "Float (single-precision)"))
  ;[0 1 0.7552] movimientp
  ;;[1 1 1] Movimiento Simplificado
  (`self.AddMovementInput` (1.0 0.0 0.0) AxisValue)
  ;;[1 1 1] Maquina de estados
  (`self.State Machine`)
  (`/Engine/EditorBlueprintResources/StandardMacros.CompareFloat` AxisValue
    (:`>`
      ;;[1 1 1] Orientacion del Personaje
      (`Controller.SetControlRotation` (`self.GetController`) (`KismetMathLibrary.MakeRotator` 0.0)))
    (:`<`
      (`Controller.SetControlRotation` (`self.GetController`) (`KismetMathLibrary.MakeRotator` 0.0 0.0 180.0)))))

(event `InputAction|salto`
  (params (Key :type "Key Structure"))
  ;[0 1 0.6746] Salto
  (:`Pressed`
    (`self.Jump`)
    (if (`NavMovementComponent.IsFalling` (`self.CharacterMovement`))
      (`self.Salto en Pared`))))

(event `self.ReceiveTick`
  (params (DeltaSeconds :type "Float (single-precision)"))
  ;[0 1 0.6499] Asignador de variables
  (if (> (`KismetMathLibrary.VSize` (`MovementComponent.Velocity` (`self.CharacterMovement`))) 0.0)
    (if (`NavMovementComponent.IsFalling` (`self.CharacterMovement`))
      (if (`self.Contacto Pared`)
        (if (`self.dash`)
          (set `self.Maquina de Estados` "NewEnumerator3")
          (else
            (set `self.Maquina de Estados` "NewEnumerator4")))
        (else
          (set `self.Maquina de Estados` "NewEnumerator2")))
      (else
        (set `self.Maquina de Estados` "NewEnumerator1")))
    (else
      (set `self.Maquina de Estados` "NewEnumerator0"))))

(event `State Machine`
  (bind _sprite (`self.Sprite`))
  ;[0 1 0.6223] Maquina de estados
  (switch `/Game/blueprints/Enumerators/e_stateMachine` (`self.Maquina de Estados`)
    (:`NewEnumerator0`
      (`PaperFlipbookComponent.SetFlipbook` _sprite null)
      (`SceneComponent.SetRelativeScale3D` _sprite (0.8 0.8 0.8)))
    (:`NewEnumerator1`
      (`PaperFlipbookComponent.SetFlipbook` _sprite "/Game/animaciones/run/run_tk.run_tk")
      (`SceneComponent.SetRelativeScale3D` _sprite (1.0 1.0 1.0)))
    (:`NewEnumerator2`
      (`PaperFlipbookComponent.SetFlipbook` _sprite "/Game/animaciones/salto2/salto2.salto2")
      (`SceneComponent.SetRelativeScale3D` _sprite (1.0 1.0 1.0)))
    (:`NewEnumerator3`
      (`PaperFlipbookComponent.SetFlipbook` _sprite "/Game/animaciones/Salto/salto_aire.salto_aire")
      (`SceneComponent.SetRelativeScale3D` _sprite (1.0 1.0 1.0)))
    (:`NewEnumerator4`
      (`PaperFlipbookComponent.SetFlipbook` _sprite "/Game/animaciones/dash/dash_per.dash_per")
      (`SceneComponent.SetRelativeScale3D` _sprite (1.0 1.0 1.0)))))

(event `Salto en Pared`
  (bind _returnvalue (`self.K2_GetActorLocation`))
  (bind _capsulecomponent (`self.CapsuleComponent`))
  (bind _capsuleradius (`CapsuleComponent.CapsuleRadius` _capsulecomponent))
  (bind _returnvalue_2 (- (`CapsuleComponent.CapsuleHalfHeight` _capsulecomponent) _capsuleradius))
  ;[0 1 0.7387] Salto en pared
  (bind (_outhit _returnvalue_3) (`KismetSystemLibrary.SphereTraceSingle` (+ _returnvalue (`KismetMathLibrary.MakeVector` _returnvalue_2)) (+ _returnvalue (`KismetMathLibrary.MakeVector` (* _returnvalue_2 -1.0))) (+ _capsuleradius 5.0) "TraceTypeQuery1"))
  (if _returnvalue_3
    (set `self.Contacto Pared` true)
    (bind (_bblockinghit _binitialoverlap _time _distance _location _impactpoint _normal _impactnormal) (`GameplayStatics.BreakHitResult` _outhit))
    (bind _returnvalue_4 (> (.x _impactnormal) 0.0))
    (`self.LaunchCharacter` (- (* (`KismetMathLibrary.GreaterGreater_VectorRotator` _impactnormal (`KismetMathLibrary.SelectRotator` (struct :`Pitch` 60.0) (struct :`Pitch` -60.0) _returnvalue_4)) (`self.Magnitud de salto`)) (`self.GetVelocity`)))
    (`Controller.SetControlRotation` (`self.GetController`) (`KismetMathLibrary.MakeRotator` 0.0 0.0 (`KismetMathLibrary.SelectFloat` 0.0 180.0 _returnvalue_4)))
    (`KismetSystemLibrary.Delay` 0.2)
    (set `self.Contacto Pared` false)))

(event `teleport`
  ;[0.305 0 0.4072] teleport
  (`self.K2_TeleportTo` (`self.K2_GetActorLocation` (`self.Referenbcia`))))

(event `Key|Q`
  (params (Key :type "Key Structure"))
  (bind _capsulecomponent (`self.CapsuleComponent`))
  ;[0.7511 0 1] dash
  (:`Pressed`
    (if (and (`self.dash`) true)
      (`self.LaunchCharacter` (`KismetMathLibrary.MakeVector` (* (`self.GetInputAxisValue`) (`self.potencia dash`))))
      (`CapsuleComponent.SetCapsuleHalfHeight` _capsulecomponent 13.0 true)
      (`KismetSystemLibrary.Delay` 0.1)
      (`CapsuleComponent.SetCapsuleHalfHeight` _capsulecomponent 31.0 true))))

(event `InputAction|inventario_imp`
  (params (Key :type "Key Structure"))
  (:`Pressed`
    (for _array_element (`self.GetOverlappingActors` "/Script/Engine.Actor")
      (if (`KismetSystemLibrary.DoesImplementInterface` _array_element "/Game/blueprints/inventario/inventario_inter.inventario_inter_C")
        (message `/Game/blueprints/inventario/inventario_inter.interact` _array_element self)
        (break)))))

(event `InputAction|abrir invetario`
  (params (Key :type "Key Structure"))
  (:`Pressed`
    (`/Game/blueprints/inventario/inventario_component.inventariofun` (`self.inventario_component`))))

(event `Key|LeftShift`
  (params (Key :type "Key Structure"))
  ;[1 1 1] Attack
  (:`Pressed`
    (`self.Attack`)
    (set `self.Ataque` true)))

(event `Attack`
  (bind _spline (`self.Spline`))
  ;[1 1 1] Attack
  (`|ExecutionSequence`
    (:`then_0`
      (bind (_direction _newtrack_0) (`Timeline|Timeline_0`)
        (:`Update`
          (bind _returnvalue (* (`SplineComponent.GetSplineLength` _spline) _newtrack_0))
          (`SceneComponent.K2_SetWorldTransform` (`self.Cube`) (`KismetMathLibrary.MakeTransform` (`SplineComponent.GetLocationAtDistanceAlongSpline` _spline _returnvalue "World") (`SplineComponent.GetRotationAtDistanceAlongSpline` _spline _returnvalue "World") (0.1 0.1 0.1)) false false))))
    (:`then_1`
      (`SceneComponent.SetVisibility` (`self.Cube`) true false))))

(event `self.CapsuleComponent.OnComponentBeginOverlap`
  (params (OverlappedComponent :type "PrimitiveComponent Object Reference") (OtherActor :type "Actor Object Reference") (OtherComp :type "PrimitiveComponent Object Reference") (OtherBodyIndex :type Integer) (bFromSweep :type Boolean) (SweepResult :type "HitResult Structure (by ref)"))
  (bind _asbolitah_sprite_bp (cast `/Game/blueprints/Bolitah_Sprite_Bp` OtherActor))
  (set `self.Enemy` _asbolitah_sprite_bp)
  (set `self.Health` (- (`self.Health`) 5.0))
  (bind _returnvalue (`|CreateWidget` "/Game/blueprints/Health_Player.Health_Player_C"))
  (`UserWidget.AddToPlayerScreen` _returnvalue 0))

(event `self.Cube.OnComponentBeginOverlap`
  (params (OverlappedComponent :type "PrimitiveComponent Object Reference") (OtherActor :type "Actor Object Reference") (OtherComp :type "PrimitiveComponent Object Reference") (OtherBodyIndex :type Integer) (bFromSweep :type Boolean) (SweepResult :type "HitResult Structure (by ref)"))
  (`|ExecutionSequence`
    (:`then_0`
      (cast `/Game/blueprints/Bolitah_Sprite_Bp` OtherActor)
      (set `self.Health_Enemy` (- (`self.Health_Enemy`) 50.0)))
    (:`then_1`
      (cast `/Game/blueprints/Enemy` OtherActor)
      (set `self.Health_Pajaro` (- (`self.Health_Pajaro`) 10.0)))))

(fn `UserConstructionScript`)