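; Patrolling 2D sprite enemy that shoots near the player and can be attacked by them.
; Tick moves it along X, reversing and mirroring the sprite at two limits, and after delays spawns a Bolitah projectile within range.
; A nearby player attack snaps the player's spline point to the enemy, destroying it once the player's HealthPajaro is depleted.
; Box overlap only casts to player_master; the player-death teleport is unconnected.
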(event `self.ReceiveBeginPlay`
  ;[1 1 1] Ref-Player
  (bind _asplayer_master (cast `/Game/blueprints/player_master` (`GameplayStatics.GetPlayerPawn` 0)))
  (set `self.Player_M` _asplayer_master))

(event `self.ReceiveTick`
  (params (DeltaSeconds :type "Float (single-precision)"))
  (bind _returnvalue_x (`KismetMathLibrary.BreakVector` (`self.K2_GetActorLocation`)))
  (bind _rendercomponent (`self.RenderComponent`))
  (bind _player_m (`self.Player_M`))
  (bind _rendercomponent_2 (`self.RenderComponent`))
  ;[1 1 1] Mov_Enemy
  (`|ExecutionSequence`
    (:`then_0`
      (`self.K2_AddActorLocalOffset` (`KismetMathLibrary.MakeVector` (`self.Movx`)))
      (if (>= _returnvalue_x (`self.Limitex`))
        (`SceneComponent.K2_SetWorldTransform` _rendercomponent_2 (`KismetMathLibrary.MakeTransform` (`SceneComponent.K2_GetComponentLocation` _rendercomponent_2) (struct) (0.1 0.1 0.1)) false false)
        (set `self.Movx` (* (`self.Movx`) -1.0) :!label _label)
        (elif (<= _returnvalue_x (`self.LimeteMenosx`))
          (`SceneComponent.K2_SetWorldTransform` _rendercomponent (`KismetMathLibrary.MakeTransform` (`SceneComponent.K2_GetComponentLocation` _rendercomponent) (struct) (-0.1 0.1 0.1)) false false)
          (goto _label))))
    (:`then_1`
      ;[1 1 1] Deteccion del Player
      (if (`KismetMathLibrary.NearlyEqual_TransformTransform` (`KismetMathLibrary.Conv_VectorToTransform` (`SceneComponent.K2_GetComponentLocation` (`self.RenderComponent`))) (`KismetMathLibrary.Conv_VectorToTransform` (`SceneComponent.K2_GetComponentLocation` (`PaperCharacter.Sprite` (`self.Player_M`)))) 200.0)
        (`KismetSystemLibrary.Delay` 1.0)
        (`|SpawnActorFromClass` "/Game/blueprints/Bolitah_Sprite_Bp.Bolitah_Sprite_Bp_C" (`KismetMathLibrary.Conv_VectorToTransform` (`SceneComponent.K2_GetComponentLocation` (`self.Arrow`))) "Undefined" "OverrideRootScale" null null)))
    (:`then_2`
      (`KismetSystemLibrary.Delay` 1.0)
      ;[1 1 1] Distancia para que el player pueda atacar al enemigo
      (if (and (`/Game/blueprints/player_master.Ataque` _player_m) (`KismetMathLibrary.NearlyEqual_TransformTransform` (`KismetMathLibrary.Conv_VectorToTransform` (`SceneComponent.K2_GetComponentLocation` (`self.RenderComponent`))) (`KismetMathLibrary.Conv_VectorToTransform` (`SceneComponent.K2_GetComponentLocation` (`PaperCharacter.Sprite` (`self.Player_M`)))) 200.0))
        (`SplineComponent.SetLocationAtSplinePoint` (`/Game/blueprints/player_master.Spline` _player_m) 1 (`SceneComponent.K2_GetComponentLocation` (`self.RenderComponent`)) "World" true)
        (`KismetSystemLibrary.PrintString` "PAJARO")
        (if (<= (`/Game/blueprints/player_master.Health_Pajaro` (`self.Player_M`)) 0.0)
          (`self.K2_DestroyActor`))))))

(event `self.Box.OnComponentBeginOverlap`
  (params (OverlappedComponent :type "PrimitiveComponent Object Reference") (OtherActor :type "Actor Object Reference") (OtherComp :type "PrimitiveComponent Object Reference") (OtherBodyIndex :type Integer) (bFromSweep :type Boolean) (SweepResult :type "HitResult Structure (by ref)"))
  ;[1 1 1] Daño Player
  (cast `/Game/blueprints/player_master` OtherActor))

(fn `UserConstructionScript`)